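; BoxButtonBP is an in-world sprite button actor with a configurable text label.
; BeginPlay enables mouse-over events on the player controller, sets the label and caches the sprite's initial color.
; While CanInteract is true, touch begin sets IsTouched and plays a click sound, and touch end clears it.
; Cursor hover sets the sprite's alpha to a fixed value, and cursor exit restores the cached color.
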(event `self.ReceiveBeginPlay`
  (set `PlayerController.bEnableMouseOverEvents` true (`GameplayStatics.GetPlayerController` 0))
  (`TextRenderComponent.K2_SetText` (`self.Option`) (`KismetTextLibrary.Conv_StringToText` (`self.text`)))
  (set `self.InitialColor` (`PaperSpriteComponent.SpriteColor` (`self.ButtonSprite`)))
  (set `self.isTouched` false))

(event `self.ReceiveActorBeginOverlap`
  (params (OtherActor :type "Actor Object Reference")))

(event `self.ReceiveTick`
  (params (DeltaSeconds :type "Float (single-precision)")))

(event `self.ReceiveActorOnInputTouchBegin`
  (params (FingerIndex :type "ETouchIndex Enum" :default "Touch1"))
  (if (`self.CanInteract`)
    (set `self.isTouched` true)
    (`GameplayStatics.PlaySound2D` "/Game/Sounds/Click1.Click1")))

(event `InputTouch`
  (params (Location :type "Vector Structure") (FingerIndex :type "ETouchIndex Enum")))

(event `self.ReceiveActorOnInputTouchEnd`
  (params (FingerIndex :type "ETouchIndex Enum" :default "Touch1"))
  (if (`self.CanInteract`)
    (set `self.isTouched` false)))

(event `self.ReceiveActorOnInputTouchEnter`
  (params (FingerIndex :type "ETouchIndex Enum" :default "Touch1")))

(event `self.ReceiveActorOnInputTouchLeave`
  (params (FingerIndex :type "ETouchIndex Enum" :default "Touch1")))

(event `self.ReceiveActorBeginCursorOver`
  (bind (_initialcolor_r _initialcolor_g _initialcolor_b) (break `LinearColor` (`self.InitialColor`)))
  (`PaperSpriteComponent.SetSpriteColor` (`self.ButtonSprite`) (make `LinearColor` _initialcolor_r _initialcolor_g _initialcolor_b 0.75)))

(event `self.ReceiveActorEndCursorOver`
  (`PaperSpriteComponent.SetSpriteColor` (`self.ButtonSprite`) (`self.InitialColor`)))

(fn `UserConstructionScript`)