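; Card back actor that shows a configurable sprite and animates its own movement and resizing.
; The construction script applies the default sprite, so it also shows in the editor viewport.
; On BeginPlay it binds lerp and resize dispatchers to events that play timelines driving location and scale.
; Each update lerps from the current transform toward the target, so motion eases rather than following the timeline alpha directly.
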(event `self.ReceiveBeginPlay`
  ;[1 1 1] Event dispatcher to lerp a card following a timeline
  (add `self.LerpCard` (delegate `MoveCard`))
  ;[1 1 1] Event dispatcher to smooth scale a card back
  (add `self.ResizeCard` (delegate `ScaleCard`)))

(event `ScaleCard` :!signature `self.ResizeCard`
  (params (`New Size` :type "Vector Structure"))
  ;[1 1 1] Event dispatcher to smooth scale a card back
  (bind (_direction _alpha) (`Timeline|Resize Timeline` :!via `PlayFromStart`)
    (:`Update`
      (`self.SetActorScale3D` (`KismetMathLibrary.VLerp` (`self.GetActorScale3D`) `New Size` _alpha)))))

(event `MoveCard` :!signature `self.LerpCard`
  (params (Destination :type "Vector Structure"))
  ;[1 1 1] Event dispatcher to lerp a card following a timeline
  (bind (_direction _alpha) (`Timeline|Timeline - Card Move` :!via `PlayFromStart`)
    (:`Update`
      (`self.OnLerp` Destination _alpha))))

(event `self.ReceiveActorBeginOverlap`
  (params (OtherActor :type "Actor Object Reference")))

(event `self.ReceiveTick`
  (params (DeltaSeconds :type "Float (single-precision)")))

(fn `OnLerp`
  (params (Target :type "Vector Structure") (Alpha :type "Float (double-precision)"))
  ;[1 1 1] Smoothly interpolates from position to another
  (`self.K2_SetActorLocation` (`KismetMathLibrary.VLerp` (`self.K2_GetActorLocation`) Target Alpha)))

(fn `UserConstructionScript`
  ;[1 1 1] Sets the sprite passed in on construction of the actor. This is preferred over on begin play because it directly modifies the sprite in the viewport tab.
  (`PaperSpriteComponent.SetSprite` (`self.MainSprite`) (`self.DefaultSprite`)))