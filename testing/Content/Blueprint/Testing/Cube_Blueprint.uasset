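; A test cube Blueprint that prints debug text according to mouse hover and left-button state.
; BeginPlay enables input from player controller 0, and Tick prints "Working" or "Not working" every frame while MouseOver is true, depending on LeftMouseHeld.
; Neither flag is set in these graphs, and a separate PrintText greeting function is never called here.
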(event `self.ReceiveBeginPlay`
  (`self.EnableInput` (`GameplayStatics.GetPlayerController` 0)))

(event `self.ReceiveActorBeginOverlap`
  (params (OtherActor :type "Actor Object Reference")))

(event `self.ReceiveTick`
  (params (DeltaSeconds :type "Float (single-precision)"))
  (if (`self.Mouse Over`)
    (if (`self.Left Mouse Held`)
      (`KismetSystemLibrary.PrintString` "Working")
      (else
        (`KismetSystemLibrary.PrintString` "Not working")))))

(fn `printText`
  (`KismetSystemLibrary.PrintString` "Hello Lucas"))

(fn `UserConstructionScript`)