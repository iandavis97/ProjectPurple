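; Heshbon card actor that shows a title derived from its data type, with a special "Lost/Found" label, plus body text.
; On BeginPlay it fills both texts and binds move, resize and rotate events to dispatchers.
; Each event plays a timeline that lerps from the current transform, compounding the easing every update.
; RotateEvent leaves its Rotation input unwired, so it lerps toward the default rotation.
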(event `self.ReceiveBeginPlay`
  (bind (_heshbondata_outcome _heshbondata_weight _heshbondata_text _heshbondata_type) (break `Heshbon` (`self.HeshbonData`)))
  (bind (_heshbondata_outcome_2 _heshbondata_weight_2 _heshbondata_text_2) (break `Heshbon` (`self.HeshbonData`)))
  ;[1 1 1] Sets Text based on type
  (switch `EHeshbonType` _heshbondata_type
    (:`None`
      (set `self.TitleText` (`KismetTextLibrary.Conv_StringToText` (`|GetEnumeratorNameAsString` _heshbondata_type)) :!label _label))
    (:`BeyondTheLaw`
      (goto _label))
    (:`LostAndFound`
      (set `self.TitleText` "Lost/Found"))
    (:`Transgression`
      (goto _label)))
  (`TextRenderComponent.K2_SetText` (`self.Title`) (`self.TitleText`))
  (`TextRenderComponent.K2_SetText` (`self.Text`) (`KismetTextLibrary.Conv_StringToText` _heshbondata_text_2))
  ;[1 1 1] Event dispatcher to lerp a card following a timeline
  (add `self.LerpCard` (delegate `MoveCard`))
  ;[1 1 1] Event dispatcher to smooth scale card
  (add `self.ResizeCard` (delegate `ScaleCard`))
  ;[1 1 1] Rotate Card
  (add `self.RotateCard` (delegate `RotateEvent`)))

(event `ScaleCard` :!signature `self.ResizeCard`
  (params (`New Size` :type "Vector Structure"))
  ;[1 1 1] Event dispatcher to smooth scale card
  (bind (_direction _alpha) (`Timeline|Scale - Timeline` :!via `PlayFromStart`)
    (:`Update`
      (`self.SetActorScale3D` (`KismetMathLibrary.VLerp` (`self.GetActorScale3D`) `New Size` _alpha)))))

(event `RotateEvent` :!signature `self.RotateCard`
  (params (Rotation :type "Vector Structure"))
  ;[1 1 1] Rotate Card
  (bind (_direction _alpha) (`Timeline|Rotate - Timeline` :!via `PlayFromStart`)
    (:`Update`
      (`self.K2_SetActorRotation` (`KismetMathLibrary.RLerp` (`self.K2_GetActorRotation`) (`KismetMathLibrary.MakeRotator` 0.0) _alpha true)))))

(event `MoveCard` :!signature `self.LerpCard`
  (params (Destination :type "Vector Structure"))
  ;[1 1 1] Event dispatcher to lerp a card following a timeline
  (bind (_direction _alpha) (`Timeline|Card Move - Timeline` :!via `PlayFromStart`)
    (:`Update`
      (`self.OnLerp` Destination _alpha))))

(fn `OnLerp`
  (params (Target :type "Vector Structure") (Alpha :type "Float (double-precision)"))
  ;[1 1 1] Smoothly interpolates from position to another
  (`self.K2_SetActorLocation` (`KismetMathLibrary.VLerp` (`self.K2_GetActorLocation`) Target Alpha)))

(fn `UserConstructionScript`)